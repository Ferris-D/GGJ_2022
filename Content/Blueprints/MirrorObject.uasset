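; MirrorObject is an actor that can be toggled in and out of the level, starting hidden with collision disabled.
; TriggerMirrorObject uses a FlipFlop to alternate the Mirrored flag on each call.
; That flag drives both actor collision and the root component's visibility, propagated to all children, so the object is either visible with collision enabled or hidden without it.
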(event `self.ReceiveBeginPlay`
  (`SceneComponent.SetVisibility` (`self.DefaultSceneRoot`) false true)
  (`self.SetActorEnableCollision` false))

(event `Trigger Mirror Object`
  (bind _mirrored (`self.Mirrored`))
  (`/Engine/EditorBlueprintResources/StandardMacros.FlipFlop`
    (:`A`
      (set `self.Mirrored` true))
    (:`B`
      (set `self.Mirrored` false)))
  (`self.SetActorEnableCollision` _mirrored)
  (`SceneComponent.SetVisibility` (`self.DefaultSceneRoot`) _mirrored true))

(fn `UserConstructionScript`)